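; BP_AI is an enemy character that can be damaged or stealth-assassinated, with a health bar that turns to face the player camera.
; Damage plays a random hit montage, launches it along the player's forward vector, shows the bar and lowers health via a stats component, ragdolling on death.
; An overlap radius toggles the assassinate prompt; StealthBackAssassin plays the victim montage, triggers a delayed ragdoll and returns alignment transforms for the attacker.
; Ragdoll disables collision, then destroys the actor.
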(event OnComponentBeginOverlap(AssassinationRadius)
  (params (OverlappedComponent :type Primitive%20Component%20Object%20Reference) (OtherActor :type Actor%20Object%20Reference) (OtherComp :type Primitive%20Component%20Object%20Reference) (OtherBodyIndex :type Integer) (bFromSweep :type Boolean) (SweepResult :type Hit%20Result%20Structure%20%28by%20ref%29))
  (Utilities|Casting|CastToBP_ThirdPersonCharacter OtherActor)
  (Rendering|SetVisibility (Variables|Default|GetAssassinate%20Widget) true false)
  (Development|PrintString "Hello"))

(event OnComponentEndOverlap(AssassinationRadius)
  (params (OverlappedComponent :type Primitive%20Component%20Object%20Reference) (OtherActor :type Actor%20Object%20Reference) (OtherComp :type Primitive%20Component%20Object%20Reference) (OtherBodyIndex :type Integer))
  (Utilities|Casting|CastToBP_ThirdPersonCharacter OtherActor)
  (Rendering|SetVisibility (Variables|Default|GetAssassinate%20Widget) false false))

(event Custom|Ragdoll
  (params (Assassinated? :type Boolean))
  ;[1 1 1] Ragdoll
  (if Assassinated?
    (Utilities|FlowControl|Delay 2.0))
  (Physics|SetSimulatePhysics (Variables|Character|GetMesh) true)
  (Audio|PlaySoundatLocation "/Game/Audio/Grunts/SC_Death.SC_Death" (Transformation|GetActorLocation) "0, 0, 0" 1.0 1.0 0.25 "/Game/Audio/SA_Character.SA_Character" 0 0 0)
  (Variables|/Script/UMG.Widget|SetVisibility (Variables|Default|GetHealthBar) "Hidden")
  (Collision|SetCollisionEnabled (Variables|Collision|GetCapsuleComponent) "NoCollision")
  (Utilities|FlowControl|Delay 1.0)
  (Actor|DestroyActor))

(event Game|Damage|EventAnyDamage
  (params (Damage :type Float%20%28single-precision%29) (DamageType :type Damage%20Type%20Object%20Reference) (InstigatedBy :type Controller%20Object%20Reference) (DamageCauser :type Actor%20Object%20Reference))
  (bind _hitanims (Variables|Default|GetHitAnims))
  (Animation|PlayAnimMontage (Utilities|Array|Get(acopy) _hitanims (Math|Random|RandomInteger (Utilities|Array|Length _hitanims))) 1.0 "None")
  (bind _asbp_third_person_character (Utilities|Casting|CastToBP_ThirdPersonCharacter (Game|GetPlayerCharacter 0)))
  (Character|LaunchCharacter (* (Math|Vector|GetForwardVector (Transformation|GetActorRotation _asbp_third_person_character)) 1e+03) false false)
  (Audio|PlaySoundatLocation "/Game/Audio/Grunts/Death2.Death2" (Transformation|GetActorLocation) "0, 0, 0" 1.0 (Math|Random|RandomFloatinRange 0.9 1.5) 0.0 "/Game/Audio/SA_Character.SA_Character" 0 0 0)
  (Variables|/Script/UMG.Widget|SetVisibility (Variables|Default|GetHealthBar) "Visible")
  (bind _isplayerdead (Default|DecreaseHealth (Variables|Default|GetBPC_PlayerStats) Damage))
  (if _isplayerdead
    (CallFunction|Ragdoll false)))

(event EventTick
  (params (DeltaSeconds :type Float%20%28single-precision%29))
  (bind _healthbarwidget (Variables|Default|GetHealthBarWidget))
  (Transformation|SetWorldRotation _healthbarwidget (Math|Rotator|FindLookatRotation (Transformation|GetWorldLocation _healthbarwidget) (Transformation|GetWorldLocation (Variables|/Script/Engine.PlayerCameraManager|GetTransformComponent (Game|GetPlayerCameraManager 0)))) false false))

(event EventBeginPlay
  (bind _aswb_dummy_health_bar (Utilities|Casting|CastToWB_DummyHealthBar (UserInterface|GetWidget (Variables|Default|GetHealthBarWidget))))
  (Variables|Default|SetHealthBar _aswb_dummy_health_bar)
  (Default|DecreaseHealth (Variables|Default|GetBPC_PlayerStats) 0.0)
  (Variables|/Script/UMG.Widget|SetVisibility (Variables|Default|GetHealthBar) "Hidden"))

(fn ConstructionScript)

(fn StealthBackAssassin
  (Animation|PlayAnimMontage "/Game/Characters/RPG_Character/Animations/Assassinations/Paired_Knife_Stealth_KidneyAndNeck_Vic_Montage.Paired_Knife_Stealth_KidneyAndNeck_Vic_Montage" 1.0 "None")
  (CallFunction|Ragdoll true)
  (Rendering|SetVisibility (Variables|Default|GetAssassinate%20Widget) false false)
  (return (Transformation|GetWorldLocation (Variables|Default|GetAssassin%20REF)) (Transformation|GetActorRotation)))