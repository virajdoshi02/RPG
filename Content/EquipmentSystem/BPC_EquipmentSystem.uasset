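; Equipment component for the third-person character that stores picked-up weapons and toggles the equipment menu.
; The menu input creates or removes the equipment widget, switching cursor and input mode and blocking attacks through the attack component while open.
; Interact sphere-traces from the follow camera, appends a hit weapon's item data to the weapon slots and destroys the actor.
; A debug key prints the stored row names.
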(event Input|EnhancedActionEvents|EnhancedInputActionIA_Interact
  (params (ActionValue :type Boolean) (ElapsedSeconds :type Float%20%28double-precision%29) (TriggeredSeconds :type Float%20%28double-precision%29) (InputAction :type Input%20Action%20Object%20Reference :default "/Game/ThirdPerson/Input/Actions/IA_Interact.IA_Interact"))
  (bind _follow_camera (Variables|Default|GetFollow%20Camera))
  (bind _returnvalue (Transformation|GetWorldLocation _follow_camera))
  ;[1 1 1] Picking up objects
  (:Started
    (bind (_outhit _returnvalue_2) (Collision|SphereTraceForObjects _returnvalue (+ (* (Math|Vector|GetForwardVector (Transformation|GetWorldRotation _follow_camera)) 8e+02) _returnvalue) 1e+01 (Utilities|Array|MakeArray "ObjectTypeQuery2") false 0 "ForDuration" true "(R=1.000000,G=0.000000,B=0.000000,A=1.000000)" "(R=0.000000,G=1.000000,B=0.000000,A=1.000000)" 0.5))
    (if _returnvalue_2
      (bind _asbp_weapon (Utilities|Casting|CastToBP_Weapon (.HitActor (Collision|BreakHitResult _outhit))))
      (CallFunction|AddWeapon (Variables|/Game/EquipmentSystem/BP_Weapon.BP_Weapon_C|GetItem%20Data _asbp_weapon))
      (Actor|DestroyActor _asbp_weapon))))

(event Input|EnhancedActionEvents|EnhancedInputActionIA_EquipmentMenu
  (params (ActionValue :type Boolean) (ElapsedSeconds :type Float%20%28double-precision%29) (TriggeredSeconds :type Float%20%28double-precision%29) (InputAction :type Input%20Action%20Object%20Reference :default "/Game/ThirdPerson/Input/Actions/IA_EquipmentMenu.IA_EquipmentMenu"))
  (bind _returnvalue (Game|GetPlayerController 0))
  (bind _bpc_attack_system (Variables|Default|GetBPC%20Attack%20System))
  ;[1 1 1] Opening GUI
  (:Started
    (if (Variables|Default|GetisPanelOpened)
      (Variables|/Game/Blueprints/BPC_AttackSystem.BPC_AttackSystem_C|SetCanAttack _bpc_attack_system true)
      (bind _equipmentwidget (Variables|Default|GetEquipmentWidget)
        (:then
          (Widget|RemovefromParent _equipmentwidget)
          (Variables|Default|SetisPanelOpened false)
          (Variables|/Script/Engine.PlayerController|SetbShowMouseCursor _returnvalue false)
          (Input|SetInputModeGameOnly _returnvalue false))
        (:else))
      (else
        (Variables|/Game/Blueprints/BPC_AttackSystem.BPC_AttackSystem_C|SetCanAttack _bpc_attack_system false)
        (bind _returnvalue_2 (UserInterface|CreateWidget "/Game/EquipmentSystem/UI/WB_Equipment.WB_Equipment_C"))
        (bind _output_get (Variables|Default|SetEquipmentWidget _returnvalue_2))
        (UserInterface|Viewport|AddtoViewport _output_get 0)
        (Variables|Default|SetisPanelOpened true)
        (Variables|/Script/Engine.PlayerController|SetbShowMouseCursor _returnvalue true)
        (Input|SetInputModeGameandUI _returnvalue (Variables|Default|GetEquipmentWidget) "DoNotLock" true false)))))

(event EventBeginPlay
  ;[1 1 1] Begin Play
  (bind _asbp_third_person_character (Utilities|Casting|CastToBP_ThirdPersonCharacter (Components|GetOwner)))
  (Variables|Default|SetFollow%20Camera (Variables|/Game/ThirdPerson/Blueprints/BP_ThirdPersonCharacter.BP_ThirdPersonCharacter_C|GetFollowCamera _asbp_third_person_character))
  (Variables|Default|SetBPC%20Attack%20System (Variables|/Game/ThirdPerson/Blueprints/BP_ThirdPersonCharacter.BP_ThirdPersonCharacter_C|GetBPC_AttackSystem _asbp_third_person_character)))

(event Input|KeyboardEvents|DebugKeyH
  (params (Key :type Key%20Structure :default "None") (ActionValue :type Input%20Action%20Value%20Structure))
  (:Pressed
    (for _array_element (Variables|Default|GetWeaponSlots)
      (Development|PrintString (Utilities|String|ToString(Name) (.RowName (Utilities|Struct|BreakDataTableRowHandle (Utilities|Struct|BreakS_Slots _array_element))))))))

(fn AddWeapon
  (params (New%20Item :type S%20Slots%20Structure%20%28by%20ref%29))
  (Utilities|Array|Add (Variables|Default|GetWeaponSlots) New%20Item))