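; Actor component that tracks health, stamina, level and XP for the third-person player character, and health for training dummies.
; BeginPlay casts the owner to set IsPlayer, routing health changes to the player HUD or the dummy's health bar.
; Stamina, max-stat and XP functions update only the player HUD, and decrease functions return whether the stat is depleted.
; IncreaseXP loops through IncreaseLevel while XP reaches MaxXP.
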(event EventBeginPlay
  (bind _returnvalue (Components|GetOwner))
  (bind _asbp_third_person_character (Utilities|Casting|CastToBP_ThirdPersonCharacter _returnvalue)
    (:then
      (Variables|Default|SetPlayerCharacter _asbp_third_person_character)
      (Variables|Default|SetisPlayer true))
    (:CastFailed
      (bind _asbp_dummy (Utilities|Casting|CastToBP_Dummy _returnvalue))
      (Variables|Default|SetDummyBP _asbp_dummy)
      (Variables|Default|SetisPlayer false))))

(fn IncreaseMaxHealth
  (params (Increase :type Float%20%28double-precision%29))
  (bind _output_get (Variables|Health|SetMaxHeath (+ (Variables|Health|GetMaxHeath) Increase)))
  (Progress|SetPercent (Variables|/Game/UI/WB_HUD.WB_HUD_C|GetHealthBar (Variables|/Game/ThirdPerson/Blueprints/BP_ThirdPersonCharacter.BP_ThirdPersonCharacter_C|GetHUD%20Widget (Variables|Default|GetPlayerCharacter))) (/ (Variables|Health|GetCurrentHealth) _output_get)))

(fn DecreaseHealth
  (params (Damage :type Float%20%28double-precision%29))
  (bind _playercharacter (Variables|Default|GetPlayerCharacter))
  (bind _hud_widget (Variables|/Game/ThirdPerson/Blueprints/BP_ThirdPersonCharacter.BP_ThirdPersonCharacter_C|GetHUD%20Widget _playercharacter))
  (if (not (<= (Variables|Health|GetCurrentHealth) 0.0))
    (bind _output_get (Variables|Health|SetCurrentHealth (- (Variables|Health|GetCurrentHealth) Damage)))
    (if (Variables|Default|GetisPlayer)
      (Progress|SetPercent (Variables|/Game/UI/WB_HUD.WB_HUD_C|GetHealthBar _hud_widget) (/ _output_get (Variables|Health|GetMaxHeath)))
      (Rendering|Components|TextRender|SetText (Variables|/Game/UI/WB_HUD.WB_HUD_C|GetHealthText _hud_widget) (Utilities|Text|ToText(Float) _output_get "HalfToEven"))
      (else
        (Progress|SetPercent (Variables|/Game/UI/WB_DummyHealthBar.WB_DummyHealthBar_C|GetHealthBar (Variables|/Game/Blueprints/BP_Dummy.BP_Dummy_C|GetHealthBar (Variables|Default|GetDummyBP))) (/ _output_get (Variables|Health|GetMaxHeath))))))
  (return (<= _output_get 0.0)))

(fn IncreaseMaxStamina
  (params (Increment :type Float%20%28double-precision%29))
  (bind _output_get (Variables|Stamina|SetMaxStamina (+ (Variables|Stamina|GetMaxStamina) Increment)))
  (Progress|SetPercent (Variables|/Game/UI/WB_HUD.WB_HUD_C|GetStaminaBar (Variables|/Game/ThirdPerson/Blueprints/BP_ThirdPersonCharacter.BP_ThirdPersonCharacter_C|GetHUD%20Widget (Variables|Default|GetPlayerCharacter))) (/ (Variables|Stamina|GetCurrentStamina) _output_get)))

(fn IncreaseStamina
  (params (Increment :type Float%20%28double-precision%29))
  (bind _output_get (Variables|Stamina|SetCurrentStamina (Math|Float|Min(Float) (+ (Variables|Stamina|GetCurrentStamina) Increment) (Variables|Stamina|GetMaxStamina))))
  (Progress|SetPercent (Variables|/Game/UI/WB_HUD.WB_HUD_C|GetStaminaBar (Variables|/Game/ThirdPerson/Blueprints/BP_ThirdPersonCharacter.BP_ThirdPersonCharacter_C|GetHUD%20Widget (Variables|Default|GetPlayerCharacter))) (/ _output_get (Variables|Stamina|GetMaxStamina))))

(fn DecreaseStamina
  (params (StaminaDepleted :type Float%20%28double-precision%29))
  (if (not (<= (Variables|Stamina|GetCurrentStamina) 0.0))
    (bind _output_get (Variables|Stamina|SetCurrentStamina (- (Variables|Stamina|GetCurrentStamina) StaminaDepleted)))
    (Progress|SetPercent (Variables|/Game/UI/WB_HUD.WB_HUD_C|GetStaminaBar (Variables|/Game/ThirdPerson/Blueprints/BP_ThirdPersonCharacter.BP_ThirdPersonCharacter_C|GetHUD%20Widget (Variables|Default|GetPlayerCharacter))) (/ _output_get (Variables|Stamina|GetMaxStamina))))
  (return (<= _output_get 0.0)))

(fn IncreaseHealth
  (params (Increment :type Float%20%28double-precision%29))
  (bind _playercharacter (Variables|Default|GetPlayerCharacter))
  (bind _hud_widget (Variables|/Game/ThirdPerson/Blueprints/BP_ThirdPersonCharacter.BP_ThirdPersonCharacter_C|GetHUD%20Widget _playercharacter))
  (bind _output_get (Variables|Health|SetCurrentHealth (Math|Float|Min(Float) (+ (Variables|Health|GetCurrentHealth) Increment) (Variables|Health|GetMaxHeath))))
  (if (Variables|Default|GetisPlayer)
    (Progress|SetPercent (Variables|/Game/UI/WB_HUD.WB_HUD_C|GetHealthBar _hud_widget) (/ _output_get (Variables|Health|GetMaxHeath)))
    (Rendering|Components|TextRender|SetText (Variables|/Game/UI/WB_HUD.WB_HUD_C|GetHealthText _hud_widget) (Utilities|Text|ToText(Float) _output_get "HalfToEven"))
    (else
      (Progress|SetPercent (Variables|/Game/UI/WB_DummyHealthBar.WB_DummyHealthBar_C|GetHealthBar (Variables|/Game/Blueprints/BP_Dummy.BP_Dummy_C|GetHealthBar (Variables|Default|GetDummyBP))) (/ _output_get (Variables|Health|GetMaxHeath))))))

(fn IncreaseLevel
  (params (Add%20Level :type Boolean))
  (Variables|XP|SetLevel (+ (Variables|XP|GetLevel) Add%20Level))
  (Variables|XP|SetXP (- (Variables|XP|GetXP) (* (Variables|XP|GetMaxXP) Add%20Level)))
  (Variables|XP|SetMaxXP (+ (Variables|XP|GetMaxXP) (* Add%20Level 1.5e+02)))
  (Rendering|Components|TextRender|SetText (Variables|/Game/UI/WB_HUD.WB_HUD_C|GetLevelText (Variables|/Game/ThirdPerson/Blueprints/BP_ThirdPersonCharacter.BP_ThirdPersonCharacter_C|GetHUD%20Widget (Variables|Default|GetPlayerCharacter))) (Utilities|Text|FormatText "{Level}" (Variables|XP|GetLevel)))
  (if Add%20Level
    (Audio|PlaySound2D "/Game/Audio/UI/Level1.Level1" 1.0 1.0 0.0 0 0)
    (Audio|PlaySound2D "/Game/Audio/UI/Level2.Level2" 1.0 1.0 0.0 0 0)))

(fn IncreaseXP
  (params (Increment :type Float%20%28double-precision%29))
  (bind _playercharacter (Variables|Default|GetPlayerCharacter))
  (bind _hud_widget (Variables|/Game/ThirdPerson/Blueprints/BP_ThirdPersonCharacter.BP_ThirdPersonCharacter_C|GetHUD%20Widget _playercharacter))
  (bind _output_get (Variables|XP|SetXP (+ Increment (Variables|XP|GetXP))))
  (if (>= _output_get (Variables|XP|GetMaxXP)) :!label _label
    (XP|IncreaseLevel false)
    (goto _label)
    (else
      (Progress|SetPercent (Variables|/Game/UI/WB_HUD.WB_HUD_C|GetXPBar _hud_widget) (/ (Variables|XP|GetXP) (Variables|XP|GetMaxXP)))
      (Rendering|Components|TextRender|SetText (Variables|/Game/UI/WB_HUD.WB_HUD_C|GetXPText _hud_widget) (Utilities|Text|FormatText "{XP} / {MaxXP}" (Variables|XP|GetXP) (Variables|XP|GetMaxXP))))))